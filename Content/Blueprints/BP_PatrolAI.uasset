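; BP_PatrolAI is an AI pawn that endlessly patrols actors tagged as patrol points for a test map.
; BeginPlay gathers and shuffles the points, randomizes walk speed, then starts GoToPatrolPoint.
; That event loops through AI MoveTo with a short delay, advancing on success or failure and reshuffling after each full pass.
; A similar GoToDestination loop chases the player character but is never called in this graph.
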(event Custom|GoToPatrolPoint
  (AI|AIMoveTo self (Transformation|GetActorLocation (Utilities|Array|Get(acopy) (stale EventBeginPlay _outactors) (Variables|Default|GetCurrentPatrolPoint))) 0 5e+01 false
    (:OnSuccess
      (Development|PrintString "Arrived at Destination" true true "(R=0.027617,G=0.196000,B=0.000000,A=1.000000)"))
    (:OnFail
      (Development|PrintString "Fail to arrive at Destination" true true "(R=1.000000,G=0.000000,B=0.000000,A=1.000000)")))
  (bind _result (Math|Integer|IncrementInt (Variables|Default|GetCurrentPatrolPoint))
    (:%20%20
      (if (>= _result (Utilities|Array|Length (stale EventBeginPlay _outactors)))
        (Variables|Default|SetCurrentPatrolPoint 0)
        (Utilities|Array|Shuffle (stale EventBeginPlay _outactors)))
      (Utilities|FlowControl|Delay 1.0)
      (CallFunction|GotoPatrolPoint))))

(event Custom|GoToDestination
  (AI|AIMoveTo self "0, 0, 0" (Game|GetPlayerCharacter 0) 5e+01 false
    (:OnSuccess
      (Development|PrintString "Arrived at Destination" true true "(R=0.027617,G=0.196000,B=0.000000,A=1.000000)"))
    (:OnFail
      (Development|PrintString "Fail to arrive at Destination" true true "(R=1.000000,G=0.000000,B=0.000000,A=1.000000)")))
  (Utilities|FlowControl|Delay 1.0)
  (CallFunction|GotoDestination))

(event EventBeginPlay
  (bind _outactors (Actor|GetAllActorsOfClasswithTag "/Script/Engine.Actor" "PatroPoint_TestMap"))
  (Development|PrintString (Utilities|String|Append "There are " (Utilities|String|ToString(Integer) (Utilities|Array|Length _outactors)) "Patrol Points"))
  (Utilities|Array|Shuffle _outactors)
  (Variables|/Script/Engine.CharacterMovementComponent|SetMaxWalkSpeed (Variables|Character|GetCharacterMovement) (Math|Conversions|ToFloat(Integer) (* (Math|Random|RandomIntegerinRange 8 12) 25)))
  (CallFunction|GotoPatrolPoint))

(fn ConstructionScript)