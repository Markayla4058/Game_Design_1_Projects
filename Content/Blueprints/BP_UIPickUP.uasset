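; BP_UIPickUP is an actor that shows a floating name label, apparently for a pickup item.
; On BeginPlay it creates a WUIPickup, assigns it to its Widget component and sets the item name text from the actor's own display name.
; A self-calling RotateTowardsPlayer event re-orients the widget every 0.1 seconds, using the look-at rotation from the player's capsule to the widget.
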(event Custom|rotate%20towards%20player
  (Transformation|SetWorldRotation (Variables|Default|GetWidget) (Math|Rotator|FindLookatRotation (Transformation|GetWorldLocation (Variables|/Script/Engine.Character|GetCapsuleComponent (Game|GetPlayerCharacter 0))) (Transformation|GetWorldLocation (Variables|Default|GetWidget))) false false)
  (Utilities|FlowControl|Delay 0.1)
  (CallFunction|RotateTowardsPlayer))

(event EventBeginPlay
  (bind _returnvalue (UserInterface|CreateWidget "/Game/Widgets/W-UIPickup.W-UIPickup_C"))
  (UserInterface|SetWidget (Variables|Default|GetWidget) _returnvalue)
  (Variables|/Script/UMG.TextBlock|SetText (Variables|/Game/Widgets/W-UIPickup.W-UIPickup_C|GetItemName _returnvalue) (Utilities|Text|ToText(String) (Utilities|GetDisplayName self)))
  (CallFunction|RotateTowardsPlayer))

(fn ConstructionScript)