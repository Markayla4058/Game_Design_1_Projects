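; BP_Spikes is a moving hazard that sends the player back to a checkpoint on contact.
; A Timeline lerps the Cone's relative location between the Start and End components.
; After each run and a fixed delay, a FlipFlop alternates between replaying forward, which comes first, and reversing.
; Overlapping the Box calls LoadCheckpoint on BP_ThirdPersonCharacterCustom.
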(event OnComponentBeginOverlap(Box)
  (params (OverlappedComponent :type Primitive%20Component%20Object%20Reference) (OtherActor :type Actor%20Object%20Reference) (OtherComp :type Primitive%20Component%20Object%20Reference) (OtherBodyIndex :type Integer) (bFromSweep :type Boolean) (SweepResult :type Hit%20Result%20Structure%20%28by%20ref%29))
  (bind _asbp_third_person_character_custom (Utilities|Casting|CastToBP_ThirdPersonCharacterCustom OtherActor))
  (Default|LoadCheckpoint _asbp_third_person_character_custom))

(event EventBeginPlay
  (bind _floattrack (Timeline|Timeline PlayFromStart)
    (:Update
      (Transformation|SetRelativeLocation (Variables|Default|GetCone) (Math|Vector|Lerp(Vector) (Variables|/Script/Engine.SceneComponent|GetRelativeLocation (Variables|Default|GetStart)) (Variables|/Script/Engine.SceneComponent|GetRelativeLocation (Variables|Default|GetEnd)) _floattrack) false false))
    (:Finished
      (Utilities|FlowControl|Delay 3.5)
      (Utilities|FlowControl|FlipFlop ; If A, Reverse from End\nif B, Start from Beginning
        (:A
          (Timeline|Timeline PlayFromStart))
        (:B
          (Timeline|Timeline ReverseFromEnd))))))

(fn ConstructionScript)